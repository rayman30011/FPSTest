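; BP_Weapon is a weapon Blueprint that provides automatic fire while its trigger state is on.
; The Fire event stores the toggle in CanFire, and when it is true spawns an actor at the skeletal mesh's MuzzleFlash socket.
; A Delay loop repeats the spawn at a fixed interval until CanFire clears, with FireDefay blocking overlapping shots during the cooldown.
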(event `Fire`
  (params (Toogle :type Boolean))
  (bind _output_get (set `self.CanFire` Toogle))
  (if _output_get
    (if (and (`self.CanFire`) (not (`self.FireDefay`))) :!label _label
      (set `self.FireDefay` true)
      (`|SpawnActorFromClass` "/Game/Blueprints/BP_Bullet.BP_Bullet_C" (`SceneComponent.GetSocketTransform` (`self.SkeletalMesh`) "MuzzleFlash" "RTS_World") "Undefined" "OverrideRootScale" null null)
      (`KismetSystemLibrary.Delay` 0.2)
      (set `self.FireDefay` false)
      (goto _label))))

(fn `UserConstructionScript`)