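; BP_AICharacter is an armed AI character that wanders the navmesh and can be killed.
; On BeginPlay it spawns a BP_Weapon and snaps it to the mesh's SKT_Gun socket.
; A Delay on Tick paces repeated AI moves to random navigable points nearby.
; TakeDamage ignores self-inflicted hits, subtracts Health, and destroys the character and its weapon once Health runs out.
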(event `/Game/Blueprints/BPI_Damagable.TakeDamage`
  (params (Value :type "Float (single-precision)") (Iniciator :type "Actor Object Reference"))
  (if (not (== Iniciator self))
    (bind _output_get (set `self.Health` (- (`self.Health`) Value)))
    (if (<= _output_get 0.0)
      (`self.K2_DestroyActor`)
      (`self.K2_DestroyActor` (`self.CurrentWeapon`)))))

(event `self.ReceiveBeginPlay`
  (`self.SnapWeapon`))

(event `self.ReceiveTick`
  (params (DeltaSeconds :type "Float (single-precision)"))
  (`KismetSystemLibrary.Delay` 2.0)
  (`|AIMoveTo` self (`NavigationSystemV1.K2_GetRandomLocationInNavigableRadius` (`self.K2_GetActorLocation`) 1000.0 null null) null))

(fn `SnapWeapon`
  (bind _returnvalue (`|SpawnActorFromClass` "/Game/Blueprints/BP_Weapon.BP_Weapon_C" (`SceneComponent.K2_GetComponentToWorld` (`self.Mesh`)) "Undefined" "OverrideRootScale" self null))
  (bind _output_get (set `self.CurrentWeapon` _returnvalue))
  (`self.K2_AttachToComponent` _output_get (`self.Mesh`) "SKT_Gun" "SnapToTarget" "SnapToTarget" "SnapToTarget" true))

(fn `UserConstructionScript`)